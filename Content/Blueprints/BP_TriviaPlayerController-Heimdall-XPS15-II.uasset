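; BP_TriviaPlayerController is a player controller that connects the trivia UI to Firebase-sourced questions.
; On BeginPlay it creates and displays WBP_TriviaUI, finds the first BP_FirebaseManager in the level, and starts the question request.
; Its OnTriviaReady event passes the received trivia to the widget if valid, with debug prints tracing the flow.
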(event Custom|OnTriviaReady
  (params (Trivia :type Trivia%20Question%20Struct%20Structure))
  (Development|PrintString "Ontrivia ready fired" true true "(R=0.000000,G=0.660000,B=1.000000,A=1.000000)" 1e+01)
  (Utilities|IsValid (Variables|Default|GetWBP_Trivia_Ref)
    (:Is%20Valid
      (Default|SetQuestionData (Variables|Default|GetWBP_Trivia_Ref) Trivia))
    (:Is%20Not%20Valid
      (Development|PrintString "Trivia Ui not ready" true true "(R=0.000000,G=0.660000,B=1.000000,A=1.000000)" 1e+01))))

(event EventBeginPlay
  (bind _returnvalue (UserInterface|CreateWidget "/Game/UI/WBP_TriviaUI.WBP_TriviaUI_C"))
  (Variables|Default|SetWBP_Trivia_Ref _returnvalue)
  (UserInterface|Viewport|AddtoViewport _returnvalue 0)
  (bind _outactors (Actor|GetAllActorsOfClass "/Game/Systems/BP_FirebaseManager.BP_FirebaseManager_C"))
  (bind _asbp_firebase_manager (Utilities|Casting|CastToBP_FirebaseManager (Utilities|Array|Get(acopy) _outactors)))
  (bind _output_get (Variables|Default|SetFirebaseManager%20Ref _asbp_firebase_manager))
  (Default|GetQuestionsfromFirebase _output_get)
  (Development|PrintString "Firebase Request Started" true true "(R=0.000000,G=0.660000,B=1.000000,A=1.000000)" 1e+01))

(event EventTick
  (params (DeltaSeconds :type Float%20%28single-precision%29)))

(fn ConstructionScript)