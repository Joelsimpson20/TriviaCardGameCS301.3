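; Game state for a multiplayer trivia game, tracking rounds and picking a category and difficulty for each.
; New rounds draw from a shrinking category pool, though pure random nodes re-roll, so the removed category can differ from the chosen one.
; A one-second retry waits for exactly two players, then multicasts an empty question.
; Work in progress: Firebase fetching is an empty stub and the multicast only casts player controllers.
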(event Custom|StartNewRound
  (Variables|Default|SetCurrentRound (+ (Variables|Default|GetCurrentRound) 1))
  (Variables|Default|SetCurrentQuestionIndex 0)
  (CallFunction|SelectRandomCatogoryandDifficulty))

(event Custom|FetchQuestionsFromFirebase)

(event Custom|Server_LoadTriviaFromGameState
  (Development|PrintString "Server load called (gamestate)" true true "(R=0.000000,G=0.660000,B=1.000000,A=1.000000)" 1e+01)
  (CallFunction|ServerFetchQuestions))

(event Custom|Multicast_ShowTriviaUI
  (params (Question :type Trivia%20Question%20Struct%20Structure))
  (Development|PrintString "Hello" true true "(R=0.000000,G=0.660000,B=1.000000,A=1.000000)" 1e+01)
  (for _array_element (Variables|Default|GetPlayerArray)
    (Utilities|IsValid _array_element
      (:Is%20Valid
        (Utilities|Casting|CastToBP_TriviaPlayerController (Game|GetPlayerController _array_element))))))

(event Custom|Server_FetchQuestions
  (CallFunction|FetchQuestionsfromFirebase))

(event Custom|WaitForAllPlayers
  (bind _playerarray (Variables|Default|GetPlayerArray))
  (bind _returnvalue (Utilities|Array|Length _playerarray))
  (Development|PrintString (Utilities|String|ToString(Integer) _returnvalue) true true "(R=0.000000,G=0.660000,B=1.000000,A=1.000000)" 0.5)
  (if (== _returnvalue 2)
    (CallFunction|MulticastShowTriviaUI (Utilities|Struct|MakeTriviaQuestionStruct (Utilities|Text|ToText(String) "") 0 (Utilities|Text|ToText(String) "")))
    (else
      (Utilities|FlowControl|Delay 1.0)
      (CallFunction|WaitforAllPlayers)
      (Development|PrintString "Player array lenggh >2 trying again"))))

(event EventBeginPlay
  (Variables|Default|SetRemainingCategories (Variables|Default|GetAllCategories)))

(event EventTick
  (params (DeltaSeconds :type Float%20%28single-precision%29)))

(fn ConstructionScript)

(fn OnRepRemainingTime)

(fn SelectRandomCatogoryandDifficulty
  (bind _remainingcategories (Variables|Default|GetRemainingCategories))
  (bind _alldifficulties (Variables|Default|GetAllDifficulties))
  (bind _returnvalue (Utilities|Array|Length _remainingcategories))
  (bind _returnvalue_2 (- _returnvalue 1))
  (bind _returnvalue_3 (Math|Random|RandomIntegerinRange 0 _returnvalue_2))
  (Variables|Default|SetCurrentCatogory (Utilities|Array|Get(acopy) _remainingcategories _returnvalue_3))
  (Utilities|Array|RemoveIndex (Variables|Default|GetRemainingCategories) _returnvalue_3)
  (Variables|Default|SetCurrentDifficulty (Utilities|Array|Get(acopy) _alldifficulties (Math|Random|RandomIntegerinRange 0 (Utilities|Array|Length _alldifficulties)))))