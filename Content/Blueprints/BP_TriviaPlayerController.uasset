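; Player controller for a trivia game that drives solo and multiplayer menus, question UI and session flow.
; Solo play opens through BP_EOSGameInstance and passes trivia to its widget, while answer checks only print the result.
; Multiplayer uses OSS account-portal login and LAN sessions: hosts open the level, joiners travel to the first session found.
; Server_HostStartGame has the game state load trivia, and Client_ShowTriviaUI displays questions in the multiplayer widget.
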(event Custom|Client_ShowTriviaUI
  (params (Question :type Trivia%20Question%20Struct%20Structure))
  ;[0.15 0.15 0.15 0.5] Client side show trivia data - checks if Muiltplayer widget refrence is vaild - adds to viewport - sets question data
  (Development|PrintString "Client Show Trivia UI Started" true true "(R=0.000000,G=0.660000,B=1.000000,A=1.000000)" 1e+01)
  (Utilities|IsValid (Variables|Default|GetMuliplayerWidgetRef)
    (:Is%20Valid
      (UserInterface|Viewport|AddtoViewport (Variables|Default|GetMuliplayerWidgetRef) 0))
    (:Is%20Not%20Valid
      (bind _returnvalue (UserInterface|CreateWidget "/Game/UI/WBP_MultiplayerTriviaUI.WBP_MultiplayerTriviaUI_C"))
      (bind _output_get (Variables|Default|SetMuliplayerWidgetRef _returnvalue))
      (Default|SetQuestionData _output_get Question)
      (UserInterface|Viewport|AddtoViewport (Variables|Default|GetMuliplayerWidgetRef) 0)
      (Development|PrintString "Multiplayer Ui created and added to viewport" true true "(R=0.000000,G=0.660000,B=1.000000,A=1.000000)" 1e+01))))

(event Custom|OnTriviaReady
  (params (Trivia :type Trivia%20Question%20Struct%20Structure))
  ;[0.15 0.15 0.15 0.5] On Trivia Ready - Calls Solo play UI - Sets Question Data
  (bind _asbp_eosgame_instance (Utilities|Casting|CastToBP_EOSGameInstance (Game|GetGameInstance)))
  (Default|ShowSoloPlay _asbp_eosgame_instance)
  (Utilities|FlowControl|Delay 1.0)
  (Default|SetQuestionData (Variables|Default|GetSoloPlayWidgetRef) Trivia))

(event Custom|OnAnswerSelected
  (params (SelectedIndex :type Integer))
  (bind _currentquestion (Variables|Default|GetCurrentQuestion))
  (bind (_question _options _answer) (Utilities|Struct|BreakTriviaQuestionStruct _currentquestion))
  ;[0.15 0.15 0.15 0.5] Answer Logic - Finds Answer for current question in struct - Compairs it to user input - Prints string
  (if (Utilities|Enum|Equal(Enum) (Utilities|Array|Get(acopy) _options SelectedIndex) _answer)
    (Development|PrintString "Correct" true true "(R=0.000000,G=0.660000,B=1.000000,A=1.000000)" 5.0)
    (else
      (Development|PrintString "Inncorect" true true "(R=0.000000,G=0.660000,B=1.000000,A=1.000000)" 5.0))))

(event Custom|AssignSoloPlayerWidget
  (params (InSoloWidget :type WBP%20Solo%20Object%20Reference))
  ;[0.15 0.15 0.15 0.5] Sets Solo Play Widget Refrence
  (Variables|Default|SetSoloPlayWidgetRef InSoloWidget))

(event Custom|ShowLobbyMenu
  (params (IsHost :type Boolean))
  ;[0.15 0.15 0.15 0.5] Show Multiplayer Lobby Menu - sets isHost
  (Variables|Default|SetIs%20Host IsHost)
  (bind _returnvalue (UserInterface|CreateWidget "/Game/UI/WBP_LobbyMenu.WBP_LobbyMenu_C"))
  (Variables|Default|SetLobbyWifgetRef _returnvalue)
  (Variables|/Game/UI/WBP_LobbyMenu.WBP_LobbyMenu_C|SetIsHost _returnvalue (Variables|Default|GetIs%20Host))
  (UserInterface|Viewport|AddtoViewport _returnvalue 0))

(event Custom|HostGame
  (|OSSCreateSession (Utilities|Map|MakeMap "MatchType" "Trivia" "MapName" "Lobby01") 2 2 false true true true false false true "LanSession" false false
    (:OnComplete
      (Variables|Default|SetOSSNicknameHost (Class|EasyOSSLibrary|GetPlayerNickName))
      (bind _asbp_eosgame_instance (Utilities|Casting|CastToBP_EOSGameInstance (Game|GetGameInstance)))
      (Variables|/Game/Blueprints/BP_EOSGameInstance.BP_EOSGameInstance_C|SetOSSNicknameHost _asbp_eosgame_instance (Variables|Default|GetOSSNicknameHost))
      (Variables|/Game/Blueprints/BP_EOSGameInstance.BP_EOSGameInstance_C|SetIsHost _asbp_eosgame_instance true)
      (Variables|/Game/Blueprints/BP_EOSGameInstance.BP_EOSGameInstance_C|SetIsBMultiplayerMenu _asbp_eosgame_instance true)
      (Game|OpenLevel(byName) "TriviaCardfGameBaseLevel")
      (Development|PrintString "Loading level" true true "(R=0.000000,G=0.660000,B=1.000000,A=1.000000)" 1e+01))
    (:OnFail
      (Development|PrintString "OSS Session Creation Failed" true true "(R=0.000000,G=0.660000,B=1.000000,A=1.000000)" 1e+01))))

(event Custom|JoinGame
  (Variables|Default|SetOSSNicknameJoiner (Class|EasyOSSLibrary|GetPlayerNickName))
  (bind _outsessions (|OSSFindSessions (Utilities|Map|MakeMap "MatchType" "Trivia" "MapName" "Lobby01") 2 "LanSession")
    (:OnSearchComplete
      (Development|PrintString "Found Session" true true "(R=0.000000,G=0.660000,B=1.000000,A=1.000000)" 1e+01)
      (Development|PrintString (Utilities|String|ToString(Name) (.SessionName (Utilities|Struct|BreakOSSSession (Utilities|Array|Get(acopy) _outsessions)))) true true "(R=0.000000,G=0.660000,B=1.000000,A=1.000000)" 1e+01)
      (bind _connectinfo (|OSSJoinSession (.SessionName (Utilities|Struct|BreakOSSSession (Utilities|Array|Get(acopy) _outsessions))) (.SessionID (Utilities|Struct|BreakOSSSession (Utilities|Array|Get(acopy) _outsessions))) "LanSession")
        (:OnComplete
          (bind _asbp_eosgame_instance (Utilities|Casting|CastToBP_EOSGameInstance (Game|GetGameInstance)))
          (Variables|/Game/Blueprints/BP_EOSGameInstance.BP_EOSGameInstance_C|SetIsBMultiplayerMenu _asbp_eosgame_instance true)
          (Variables|/Game/Blueprints/BP_EOSGameInstance.BP_EOSGameInstance_C|SetIsHost _asbp_eosgame_instance false)
          (Development|PrintString "Joined Session " true true "(R=0.000000,G=0.660000,B=1.000000,A=1.000000)" 1e+01)
          (Class|EasyOSSLibrary|DoClientTravel (Game|GetPlayerController 0) _connectinfo "TRAVEL_Absolute" false)
          (Development|PrintString "Client Travled")
          (bind _returnvalue (UserInterface|CreateWidget "/Game/UI/WBP_LobbyMenu.WBP_LobbyMenu_C"))
          (UserInterface|Viewport|AddtoViewport _returnvalue 0)
          (bind _aswbp_lobby_menu (Utilities|Casting|CastToWBP_LobbyMenu (Variables|Default|GetLobbyWifgetRef)))
          (Default|RefreshLobbyNames _aswbp_lobby_menu))))
    (:OnSearchFail
      (Development|PrintString "no session found"))))

(event Custom|Server_HostStartGame
  (bind _asbp_trivia_game_state (Utilities|Casting|CastToBP_TriviaGameState (Game|GetGameState)))
  (Default|ServerLoadTriviafromGameState _asbp_trivia_game_state))

(event Custom|LoginToEOS
  (|OSSLoginPlayer (Utilities|Struct|MakeOSSOnlineAccountCredentials "AccountPortal")
    (:OnComplete
      (bind _returnvalue (UserInterface|CreateWidget "/Game/UI/WBP_Multiplayer.WBP_Multiplayer_C"))
      (UserInterface|Viewport|AddtoViewport _returnvalue 0)
      (Development|PrintString "OSS Login Success" true true "(R=0.000000,G=0.660000,B=1.000000,A=1.000000)" 1e+01)
      (Development|PrintString (Class|EasyOSSLibrary|GetPlayerUniqueID) true true "(R=0.000000,G=0.660000,B=1.000000,A=1.000000)" 3e+01))
    (:OnFail
      (Development|PrintString "Failed to Login to OSS" true true "(R=0.000000,G=0.660000,B=1.000000,A=1.000000)" 1e+01))))

(event EventBeginPlay
  ;[0.15 0.15 0.15 0.5] BeginPlay - Sets Mouse Cursor - Calls Main Menu UI
  (Variables|Default|SetbShowMouseCursor true)
  (bind _asbp_eosgame_instance (Utilities|Casting|CastToBP_EOSGameInstance (Game|GetGameInstance)))
  (Default|ShowMainMenu _asbp_eosgame_instance))

(fn ConstructionScript)