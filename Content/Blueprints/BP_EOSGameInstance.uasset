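; Game instance for a trivia game that creates and shows its main, solo, multiplayer and lobby menus.
; Opening the multiplayer menu runs once and sets a flag that makes ShowMainMenu show the lobby, passing host status.
; Otherwise the main menu shows once, with UI-only input when newly created.
; Solo play hands its new widget to BP_TriviaPlayerController, but never stores it in the SoloPlayWidget variable it checks.
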(fn ShowMainMenu
  (if (Variables|Default|GetIsBMultiplayerMenu)
    (bind _returnvalue (UserInterface|CreateWidget "/Game/UI/WBP_LobbyMenu.WBP_LobbyMenu_C" (Game|GetPlayerController 0) (Variables|Default|GetIsHost)))
    (UserInterface|Viewport|AddtoViewport _returnvalue 0)
    (else
      (Utilities|FlowControl|DoOnce false
        (:Completed
          (Utilities|IsValid (Variables|Default|GetMainMenuWidget)
            (:Is%20Valid
              (UserInterface|Viewport|AddtoViewport (Variables|Default|GetMainMenuWidget) 0))
            (:Is%20Not%20Valid
              (bind _returnvalue_2 (UserInterface|CreateWidget "/Game/UI/WBP_MainMenu.WBP_MainMenu_C" (Game|GetPlayerController 0)))
              (bind _output_get (Variables|Default|SetMainMenuWidget _returnvalue_2))
              (UserInterface|Viewport|AddtoViewport _output_get 0)
              (Input|SetInputModeUIOnly (Game|GetPlayerController 0) (Variables|Default|GetMainMenuWidget) "DoNotLock" false))))))))

(fn ShowSoloPlay
  (Utilities|IsValid (Variables|Default|GetSoloPlayWidget)
    (:Is%20Valid
      (UserInterface|Viewport|AddtoViewport (Variables|Default|GetSoloPlayWidget) 0))
    (:Is%20Not%20Valid
      (bind _returnvalue (UserInterface|CreateWidget "/Game/UI/WBP_Solo.WBP_Solo_C" (Game|GetPlayerController 0)))
      (UserInterface|Viewport|AddtoViewport _returnvalue 0)
      (bind _asbp_trivia_player_controller (Utilities|Casting|CastToBP_TriviaPlayerController (Game|GetPlayerController 0)))
      (Default|AssignSoloPlayerWidget _asbp_trivia_player_controller _returnvalue))))

(fn ShowMultioplayerMenu
  (Utilities|FlowControl|DoOnce false
    (:Completed
      (bind _returnvalue (UserInterface|CreateWidget "/Game/UI/WBP_Multiplayer.WBP_Multiplayer_C" (Class|GameplayStatics|GetPlayerControllerfromID)))
      (UserInterface|Viewport|AddtoViewport _returnvalue 0)
      (Variables|Default|SetIsBMultiplayerMenu true))))