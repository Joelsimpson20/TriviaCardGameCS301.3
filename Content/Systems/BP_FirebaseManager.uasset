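; Firebase manager for the trivia game that fetches questions from a Realtime Database and hands one to the player controller.
; RequestTriviaData sends a VaRest GET to a URL built from category and difficulty.
; OnFirebaseResponse turns only the response's first entry into a question struct with text, four options and answer.
; It passes this to BP_TriviaPlayerController's OnTriviaReady, then sets CurrentQuestion afterwards.
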(event Custom|RequestTriviaData
  (params (Category :type Text) (Difficulty :type Text))
  (CallFunction|GetQuestionsfromFirebase Category Difficulty))

(event Custom|OnFirebaseResponse
  (params (Request :type %20Object%20Reference))
  (bind _returnvalue (CallFunction|GetResponseObject))
  (bind _returnvalue_2 (CallFunction|GetFieldNames _returnvalue))
  (bind _output (Utilities|Array|Get(acopy) _returnvalue_2))
  (bind _returnvalue_3 (CallFunction|GetObjectField _returnvalue _output))
  (bind _returnvalue_4 (CallFunction|GetStringArrayField _returnvalue_3 "options"))
  (bind _returnvalue_5 (CallFunction|GetStringField _returnvalue_3 "text"))
  (bind _returnvalue_6 (CallFunction|GetStringField _returnvalue_3 "answer"))
  (bind _returnvalue_7 (Utilities|Text|ToText(String) _returnvalue_6))
  (bind _returnvalue_8 (Utilities|Text|ToText(String) _returnvalue_5))
  (bind _output_2 (Utilities|Array|Get(acopy) _returnvalue_4))
  (bind _output_3 (Utilities|Array|Get(acopy) _returnvalue_4 1))
  (bind _output_4 (Utilities|Array|Get(acopy) _returnvalue_4 2))
  (bind _output_5 (Utilities|Array|Get(acopy) _returnvalue_4 3))
  (bind _returnvalue_9 (|GenerictoText _output_5))
  (bind _returnvalue_10 (|GenerictoText _output_2))
  (bind _returnvalue_11 (|GenerictoText _output_3))
  (bind _returnvalue_12 (|GenerictoText _output_4))
  (bind _array (Utilities|Array|MakeArray _returnvalue_10 _returnvalue_11 _returnvalue_12 _returnvalue_9))
  (bind _triviaquestionstruct (Utilities|Struct|MakeTriviaQuestionStruct _returnvalue_8 _array _returnvalue_7))
  (bind _asbp_trivia_player_controller (Utilities|Casting|CastToBP_TriviaPlayerController (Game|GetPlayerController 0)))
  (Default|OnTriviaReady _asbp_trivia_player_controller _triviaquestionstruct)
  (Variables|/Game/Blueprints/BP_TriviaPlayerController.BP_TriviaPlayerController_C|SetCurrentQuestion _asbp_trivia_player_controller _triviaquestionstruct))

(event EventBeginPlay)

(fn ConstructionScript)

(fn GetQuestionsfromFirebase
  (params (category :type Text) (difficulty :type Text))
  (bind _returnvalue (CallFunction|ConstructVaRestRequest (|EngineSubsystem)))
  (EventDispatchers|BindEventtoOnRequestComplete _returnvalue (EventDispatchers|CreateEvent :!event Custom|OnFirebaseResponse))
  (CallFunction|SetVerb _returnvalue 0)
  (CallFunction|SetURL _returnvalue (Utilities|String|Append (Utilities|String|Append (Utilities|String|Append (Utilities|String|Append "https://triviacardgame-e0a97-default-rtdb.asia-southeast1.firebasedatabase.app/questions/" (Utilities|String|ToString(Text) category)) "/") (Utilities|String|ToString(Text) difficulty)) ".json"))
  (Development|PrintString "Exe Firebase Request" true true "(R=0.000000,G=0.660000,B=1.000000,A=1.000000)" 1e+01)
  (CallFunction|ExecuteProcessRequest _returnvalue))

(fn NewFunction)

(fn GetResponseObject)